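; Game mode for a match with players and bots, tracking kills, deaths and collected Sun Pillars.
; BeginPlay spawns the game instance's bot count and counts pillars; bots and restarted players move to random reachable points around a PlayerStart.
; Player deaths trigger CheckWinner, which judges by alive status (returning a survivor when AliveCount is not 1) or full pillar collection.
; EndGame multicasts winner and top-killer results through BP_GameState.
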(event `self.K2_OnRestartPlayer`
  (params (NewPlayer :type "Controller Object Reference"))
  (bind _asbp_player (cast `/Game/Blueprints/Game/Characters/Player/BP_Player` (`Controller.K2_GetPawn` NewPlayer)))
  (`self.MoveAtRandomLocation` _asbp_player))

(event `self.ReceiveBeginPlay`
  (`|ExecutionSequence`
    (:`then_0`
      ; Game Settings
      (bind _asbp_game_instance (cast `/Game/Blueprints/BP_GameInstance` (`GameplayStatics.GetGameInstance`)))
      (set `self.NpcSpawnCount` (`/Game/Blueprints/BP_GameInstance.MaxBotCount` _asbp_game_instance)))
    (:`then_1`
      ; Spawn Npc
      (`self.SpawnNpc` (`self.NpcSpawnCount`)))
    (:`then_2`
      ; Spawn Sun Pilaras
      (bind _outactors (`GameplayStatics.GetAllActorsOfClass` "/Game/Blueprints/Game/Env/BP_SunPillar.BP_SunPillar_C"))
      (set `self.SunPillarCount` (`KismetArrayLibrary.Array_Length` _outactors)))
    (:`then_3`
      (set `self.bUseSeamlessTravel` true))))

(fn `CheckWinner`
  (if (not (`self.IsGameOver`))
    (`/Engine/EditorBlueprintResources/StandardMacros.IsValid` (`self.GetWinner`)
      (:`Is Valid`
        (`|ExecutionSequence`
          (:`then_0`
            (set `self.IsGameOver` true))
          (:`then_1`
            (`self.EndGame`)))))))

(fn `EndGame`
  (bind _player (`self.GetMostKillPlayer`))
  ; GameEnd
  (bind _asbp_game_state (cast `/Game/Blueprints/Game/BP_GameState` (`GameplayStatics.GetGameState`)))
  (`/Game/Blueprints/Game/BP_GameState.Multicast_GameResult` _asbp_game_state (`/Game/Blueprints/Game/Characters/Player/BP_PlayerState.Nickname` (`self.GetWinner`)) (`/Game/Blueprints/Game/Characters/Player/BP_PlayerState.Nickname` _player) (`/Game/Blueprints/Game/Characters/Player/BP_PlayerState.Kills` _player)))

(fn `GetMostKillPlayer`
  (returns (Player :type "/Game/Blueprints/Game/Characters/Player/BP_PlayerState Object Reference"))
  (locals (LocalBestKills :type Integer :default -1) (LocalBestPlayer :type "/Game/Blueprints/Game/Characters/Player/BP_PlayerState Object Reference"))
  (bind _localbestkills (`local.LocalBestKills`))
  (`|ExecutionSequence`
    (:`then_0`
      ; GetMostKillPlayer
      (for _array_element (`GameStateBase.PlayerArray` (`GameplayStatics.GetGameState`))
        (bind _asbp_player_state (cast `/Game/Blueprints/Game/Characters/Player/BP_PlayerState` _array_element))
        (if (> (`/Game/Blueprints/Game/Characters/Player/BP_PlayerState.Kills` _asbp_player_state) _localbestkills)
          (set `local.LocalBestKills` _localbestkills)
          (set `local.LocalBestPlayer` _asbp_player_state))))
    (:`then_1`
      ; Return Best Player
      (return (`local.LocalBestPlayer`)))))

(fn `GetWinner`
  (returns (OutWinner :type "/Game/Blueprints/Game/Characters/Player/BP_PlayerState Object Reference"))
  (locals (AliveCount :type Integer))
  (`|ExecutionSequence`
    (:`then_0`
      ; Alive Count
      (for _array_element (`GameStateBase.PlayerArray` (`GameplayStatics.GetGameState`))
        (bind _asbp_player_state (cast `/Game/Blueprints/Game/Characters/Player/BP_PlayerState` _array_element))
        (if (not (`/Game/Blueprints/Game/Characters/Player/BP_PlayerState.IsDead` _asbp_player_state))
          (`/Engine/EditorBlueprintResources/StandardMacros.IncrementInt` (`local.AliveCount`)))))
    (:`then_1`
      ; GetWinner (IsAlive)
      (if (not (== (`local.AliveCount`) 1))
        (for _array_element_2 (`GameStateBase.PlayerArray` (`GameplayStatics.GetGameState`))
          (bind _asbp_player_state_2 (cast `/Game/Blueprints/Game/Characters/Player/BP_PlayerState` _array_element_2))
          (if (not (`/Game/Blueprints/Game/Characters/Player/BP_PlayerState.IsDead` _asbp_player_state_2))
            (return _asbp_player_state_2)))))
    (:`then_2`
      ; GetWinner (SunPillar)
      (if (> (`self.SunPillarCount`) 0)
        (for _array_element_3 (`GameStateBase.PlayerArray` (`GameplayStatics.GetGameState`))
          (bind _asbp_player_state_3 (cast `/Game/Blueprints/Game/Characters/Player/BP_PlayerState` _array_element_3))
          (if (== (`BlueprintSetLibrary.Set_Length` (`/Game/Blueprints/Game/Characters/Player/BP_PlayerState.SunPillars` _asbp_player_state_3)) (`self.SunPillarCount`))
            (return _asbp_player_state_3)))))
    (:`then_3`
      (return null))))

(fn `MoveAtRandomLocation`
  (params (InActor :type "Actor Object Reference"))
  (bind _returnvalue (`GameplayStatics.GetActorOfClass` "/Script/Engine.PlayerStart"))
  (bind (_randomlocation _returnvalue_2) (`NavigationSystemV1.K2_GetRandomReachablePointInRadius` (`self.K2_GetActorLocation` _returnvalue) 50000.0 null null))
  (if _returnvalue_2
    (`self.K2_SetActorLocation` _randomlocation)))

(fn `OnPlayerDeath`
  (params (InPlayerState :type "/Game/Blueprints/Game/Characters/Player/BP_PlayerState Object Reference"))
  ; On Player Death
  (set `/Game/Blueprints/Game/Characters/Player/BP_PlayerState.IsDead` true InPlayerState)
  (`self.CheckWinner`))

(fn `OnStickmanDeath`
  (params (InAttacker :type "/Game/Blueprints/Game/Characters/Player/BP_Player Object Reference") (InVictim :type "/Game/Blueprints/Game/Characters/BP_Stickman Object Reference"))
  (bind _playersate (`/Game/Blueprints/Game/Characters/Player/BP_Player.GetBP_PlayerState` (`local.InAttacker`)))
  (`/Engine/EditorBlueprintResources/StandardMacros.IsValid` InAttacker
    (:`Is Valid`
      (`/Engine/EditorBlueprintResources/StandardMacros.IsValid` InVictim
        (:`Is Valid`
          (`|ExecutionSequence`
            (:`then_0`
              ; Add KillCount
              (`/Engine/EditorBlueprintResources/StandardMacros.IsValid` _playersate
                (:`Is Valid`
                  (`/Engine/EditorBlueprintResources/StandardMacros.IncrementInt` (`/Game/Blueprints/Game/Characters/Player/BP_PlayerState.Kills` _playersate)))))
            (:`then_1`
              ; OnPlayerDeath
              (bind _asbp_player (cast `/Game/Blueprints/Game/Characters/Player/BP_Player` (`local.InVictim`)))
              (`self.OnPlayerDeath` (`/Game/Blueprints/Game/Characters/Player/BP_Player.GetBP_PlayerState` _asbp_player)))))))))

(fn `OnTriggerSunPillar`
  (params (InPlayerState :type "/Game/Blueprints/Game/Characters/Player/BP_PlayerState Object Reference") (InSunPillar :type "/Game/Blueprints/Game/Env/BP_SunPillar Object Reference"))
  (`/Engine/EditorBlueprintResources/StandardMacros.IsValid` InPlayerState
    (:`Is Valid`
      (`/Engine/EditorBlueprintResources/StandardMacros.IsValid` InSunPillar
        (:`Is Valid`
          (`|ExecutionSequence`
            (:`then_0`
              ; Add SunPillar
              (if (not (`BlueprintSetLibrary.Set_Contains` (`/Game/Blueprints/Game/Characters/Player/BP_PlayerState.SunPillars` (`local.InPlayerState`)) (`local.InSunPillar`)))
                (`BlueprintSetLibrary.Set_Add` (`/Game/Blueprints/Game/Characters/Player/BP_PlayerState.SunPillars` (`local.InPlayerState`)) (`local.InSunPillar`))))))))))

(fn `SpawnNpc`
  (params (InSpawnCount :type Integer))
  (for _ (range 1 (+ InSpawnCount 1))
    (bind _returnvalue (`|SpawnActorFromClass` "/Game/Blueprints/Game/Characters/NPC/BP_Npc.BP_Npc_C" (`KismetMathLibrary.MakeTransform` (0.0 0.0 0.0)) "AdjustIfPossibleButAlwaysSpawn" "MultiplyWithRoot" null null))
    (`self.MoveAtRandomLocation` _returnvalue)))

(fn `UserConstructionScript`)