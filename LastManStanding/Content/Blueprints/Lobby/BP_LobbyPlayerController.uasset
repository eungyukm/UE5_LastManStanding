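; Lobby player controller that relays a player's ready and nickname requests from the lobby to the server.
; Each handler calls a server event, which acts on the BP_LobbyPlayerState of the controlled pawn.
; Readying triggers the player state's MulticastReady, then asks BP_LobbyGameMode to try starting the game.
; A nickname change writes the new name directly to the player state on the server.
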(event `HandleReadyButton`
  ;[1 1 1] Ready Button
  (`self.Server_handleReadyButton`))

(event `Server_HandleReadyButton`
  ;[1 1 1] Ready Button
  (if (`KismetSystemLibrary.IsServer`)
    (bind _asbp_lobby_player_state (cast `/Game/Blueprints/Lobby/BP_LobbyPlayerState` (`Pawn.PlayerState` (`self.K2_GetPawn`))))
    (`/Game/Blueprints/Lobby/BP_LobbyPlayerState.Multicast_Ready` _asbp_lobby_player_state)
    (bind _asbp_lobby_game_mode (cast `/Game/Blueprints/Lobby/BP_LobbyGameMode` (`GameplayStatics.GetGameMode`)))
    (`/Game/Blueprints/Lobby/BP_LobbyGameMode.TryStartGame` _asbp_lobby_game_mode)))

(event `HandleChangeNickName`
  (params (InNickName :type Text))
  ;[1 1 1] Change Nickname
  (`self.Server_HandleChangeNickName` InNickName))

(event `Server_HandleChangeNickName`
  (params (InNickName :type Text))
  ;[1 1 1] Change Nickname
  (if (`KismetSystemLibrary.IsServer`)
    (bind _asbp_lobby_player_state (cast `/Game/Blueprints/Lobby/BP_LobbyPlayerState` (`Pawn.PlayerState` (`self.K2_GetPawn`))))
    (set `/Game/Blueprints/Lobby/BP_LobbyPlayerState.Nickname` InNickName _asbp_lobby_player_state)))

(fn `UserConstructionScript`)