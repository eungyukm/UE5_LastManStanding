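; Lobby game mode that names joining players, stores match settings and starts the game by changing level.
; PostLogin assigns numbered "User" nicknames on the lobby PlayerState, and SaveConfig stores player and bot limits plus the chosen map's level name.
; TryStartGame runs a delayed travel console command once IsEverybodyReady passes.
; That function's Ready check is disconnected, so it only casts player states, never testing readiness.
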(event `self.K2_PostLogin`
  (params (NewPlayer :type "PlayerController Object Reference"))
  (bind _asbp_lobby_player_state (cast `/Game/Blueprints/Lobby/BP_LobbyPlayerState` (`Controller.PlayerState` NewPlayer)))
  (bind _result (`/Engine/EditorBlueprintResources/StandardMacros.IncrementInt` (`self.NicknameIndex`))
    (:`  `
      (set `/Game/Blueprints/Lobby/BP_LobbyPlayerState.Nickname` (`|FormatText` "User{0}" _result) _asbp_lobby_player_state))))

(event `TryStartGame`
  (if (`self.IsEverybodyReady`)
    (`KismetSystemLibrary.Delay` 1.0)
    (`KismetSystemLibrary.ExecuteConsoleCommand` (`KismetStringLibrary.Concat_StrStr` "Server Travel" "" (`self.LevelName`)) null)))

(fn `IsEverybodyReady`
  (returns (Ready :type Boolean))
  ; IsEverybodyReady
  (for _array_element (`GameStateBase.PlayerArray` (`GameplayStatics.GetGameState`))
    (bind _asbp_lobby_player_state (cast `/Game/Blueprints/Lobby/BP_LobbyPlayerState` _array_element)))
  (return true))

(fn `SaveConfig`
  (params (InLevelName :type String) (InMaxPlayerCount :type Integer) (InMaxBotCount :type Integer))
  ; SaveConfig
  (`|ExecutionSequence`
    (:`then_0`
      (switch `string` (`local.InLevelName`)
        (:`Default`
          (set `self.LevelName` "Level_WaterWheel" :!label _label))
        (:`Fountain`
          (set `self.LevelName` "Level_Fountain"))
        (:`Watermill`
          (goto _label))))
    (:`then_1`
      (set `self.MaxPlayerCount` (`local.InMaxPlayerCount`)))
    (:`then_2`
      (set `self.MaxBotCount` (`local.InMaxBotCount`)))))

(fn `UserConstructionScript`)