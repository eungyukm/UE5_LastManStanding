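; Lobby player state that keeps the lobby UI in step with each player's presence, nickname and ready status.
; BeginPlay, destruction, the Nickname RepNotify and the multicast Ready event all call RefreshLobbyUI, which tells the local player controller's BP_LobbyHUD to refresh.
; A client event for being kicked by the server opens the Title level.
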(event `Client_KickedByServer`
  (`GameplayStatics.OpenLevelBySoftObjectPtr` "/Game/Maps/Title.Title"))

(event `Multicast_Ready`
  (set `self.Ready` true)
  (`self.RefreshLobbyUI`))

(event `self.ReceiveBeginPlay`
  (`self.RefreshLobbyUI`)
  (add `self.OnDestroyed` (delegate `OnDestroyed_Event`) :!label _label))

(event `OnDestroyed_Event` :!signature `self.OnDestroyed`
  (params (DestroyedActor :type "Actor Object Reference"))
  (`self.RefreshLobbyUI`)
  (goto _label))

(fn `OnRep_Nickname`
  (`self.RefreshLobbyUI`))

(fn `RefreshLobbyUI`
  (bind _returnvalue (`GameplayStatics.GetPlayerController` 0))
  ; Refresh Ready UI
  (`/Engine/EditorBlueprintResources/StandardMacros.IsValid` _returnvalue
    (:`Is Valid`
      (bind _asbp_lobby_hud (cast `/Game/Blueprints/Lobby/BP_LobbyHUD` (`PlayerController.GetHUD` _returnvalue)))
      (`/Game/Blueprints/Lobby/BP_LobbyHUD.RefreshUI` _asbp_lobby_hud))))

(fn `UserConstructionScript`)